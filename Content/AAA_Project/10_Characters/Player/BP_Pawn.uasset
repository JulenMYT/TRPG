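; BP_Pawn is the player pawn for tactical mode, acting as a camera with movement, zoom and stepped rotation.
; BeginPlay adds the tactical input mapping context and seeds desired location, rotation and arm length from current values.
; Enhanced Input events only update those targets, moving relative to pawn facing, clamping zoom and stepping yaw once per press.
; Tick interpolates the actor transform and spring arm length toward the targets for smooth motion, without sweep.
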(event Input|EnhancedActionEvents|EnhancedInputActionIA_Zoom
  (params (ActionValue :type Float%20%28double-precision%29) (ElapsedSeconds :type Float%20%28double-precision%29) (TriggeredSeconds :type Float%20%28double-precision%29) (InputAction :type Input%20Action%20Object%20Reference :default "/Game/AAA_Project/00_Core/Inputs/IA_Zoom.IA_Zoom"))
  ;[0.15 0.15 0.15 0.5] Zoom
  (Variables|Default|SetZoomDesired (Math|Float|Clamp(Float) (+ (Variables|Default|GetZoomDesired) (* ActionValue (Variables|Default|GetZoomSpeed))) (Variables|Default|GetZoomMin) (Variables|Default|GetZoomMax))))

(event Input|EnhancedActionEvents|EnhancedInputActionIA_Move
  (params (ActionValue :type Vector%202D%20Structure) (ElapsedSeconds :type Float%20%28double-precision%29) (TriggeredSeconds :type Float%20%28double-precision%29) (InputAction :type Input%20Action%20Object%20Reference :default "/Game/AAA_Project/00_Core/Inputs/IA_Move.IA_Move"))
  (bind _locationspeed (Variables|Default|GetLocationSpeed))
  ;[0.15 0.15 0.15 0.5] Location
  (Variables|Default|SetLocationDesired (+ (+ (Variables|Default|GetLocationDesired) (* (* (.x ActionValue) _locationspeed) (Transformation|GetActorForwardVector))) (* (* (.y ActionValue) _locationspeed) (Transformation|GetActorRightVector)))))

(event Input|EnhancedActionEvents|EnhancedInputActionIA_RotateLeft
  (params (ActionValue :type Boolean) (ElapsedSeconds :type Float%20%28double-precision%29) (TriggeredSeconds :type Float%20%28double-precision%29) (InputAction :type Input%20Action%20Object%20Reference :default "/Game/AAA_Project/00_Core/Inputs/IA_RotateLeft.IA_RotateLeft"))
  ;[0.15 0.15 0.15 0.5] Rotation
  (:Started
    (Variables|Default|SetRotationDesired (Math|Rotator|CombineRotators (Variables|Default|GetRotationDesired) (Math|Rotator|MakeRotator 0.0 0.0 (Variables|Default|GetRotationSpeed))))))

(event Input|EnhancedActionEvents|EnhancedInputActionIA_RotateRight
  (params (ActionValue :type Boolean) (ElapsedSeconds :type Float%20%28double-precision%29) (TriggeredSeconds :type Float%20%28double-precision%29) (InputAction :type Input%20Action%20Object%20Reference :default "/Game/AAA_Project/00_Core/Inputs/IA_RotateRight.IA_RotateRight"))
  ;[0.15 0.15 0.15 0.5] Rotation
  (:Started
    (Variables|Default|SetRotationDesired (Math|Rotator|CombineRotators (Variables|Default|GetRotationDesired) (Math|Rotator|MakeRotator 0.0 0.0 (- 0.0 (Variables|Default|GetRotationSpeed)))))))

(event EventTick
  (params (DeltaSeconds :type Float%20%28single-precision%29))
  (bind _springarm (Variables|Default|GetSpringArm))
  (Variables|/Script/Engine.SpringArmComponent|SetTargetArmLength _springarm (Math|Interpolation|FInterpTo (Variables|/Script/Engine.SpringArmComponent|GetTargetArmLength _springarm) (Variables|Default|GetZoomDesired) DeltaSeconds (Variables|Default|GetZoomInterp)))
  (Transformation|SetActorLocation (Math|Interpolation|VInterpTo (Transformation|GetActorLocation) (Variables|Default|GetLocationDesired) DeltaSeconds (Variables|Default|GetLocationInterp)) false false)
  (Transformation|SetActorRotation (Math|Interpolation|RInterpTo (Transformation|GetActorRotation) (Variables|Default|GetRotationDesired) DeltaSeconds (Variables|Default|GetRotationInterp))))

(event EventBeginPlay
  (Input|AddMappingContext (PlayerController|LocalPlayerSubsystems|GetEnhancedInputLocalPlayerSubsystem (Game|GetPlayerController 0)) "/Game/AAA_Project/00_Core/Inputs/IMC_TacticalMode.IMC_TacticalMode" 0 "(bIgnoreAllPressedKeysUntilRelease=True,bForceImmediately=False,bNotifyUserSettings=False)")
  (Variables|Default|SetLocationDesired (Transformation|GetActorLocation))
  (Variables|Default|SetZoomDesired (Variables|/Script/Engine.SpringArmComponent|GetTargetArmLength (Variables|Default|GetSpringArm)))
  (Variables|Default|SetRotationDesired (Transformation|GetActorRotation)))

(fn ConstructionScript)