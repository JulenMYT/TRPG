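; Grid-based tactics unit actor that loads mesh, anim and stats from its unit type, holds HP/MP/AP and shows team color on an HP bar and tile marker.
; A timeline walks it tile by tile along a path, broadcasting movement events.
; Spell casts spend AP; hits change HP immediately but defer bar, number and animation feedback until the spell animation reaches its tile.
; MP and AP refill at combat start, turn end and combat end.
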(event Custom|Event_FollowPath
  (params (Path :type Array%20of%20Int%20Point%20Structures))
  (if (> (Utilities|Array|Length Path) 0)
    (Variables|UnitMovement|SetCurrent%20Path%20To%20Follow Path)
    (Default|CallOnUnitStartedWalking self)
    (CallFunction|ContinuetoFollowPath)))

(event Custom|ContinueToFollowPath
  (bind _grid (Variables|Grid|GetGrid))
  (bind _timeline_unitmovement (Variables|Default|GetTimeline_UnitMovement))
  (bind _current_path_to_follow (Variables|UnitMovement|GetCurrent%20Path%20To%20Follow))
  (bind _output (Utilities|Array|Get(acopy) _current_path_to_follow))
  (bind _gridtiles (Variables|/Game/AAA_Project/00_Core/Grid/BP_Grid.BP_Grid_C|GetGridTiles _grid))
  (bind _value (Utilities|Map|Find _gridtiles _output))
  (bind _transform (Utilities|Struct|BreakS_TileData _value))
  (if (> (Utilities|Array|Length (Variables|UnitMovement|GetCurrent%20Path%20To%20Follow)) 0)
    (Animation|SetAnimationState "NewEnumerator1")
    (Variables|UnitMovement|SetPrevious%20Transform (Transformation|GetActorTransform))
    (Variables|UnitMovement|SetNext%20Transform (Math|Transform|MakeTransform (.location _transform) (Math|Rotator|MakeRotator 0.0 0.0 (.yaw (Math|Rotator|FindLookatRotation (.location (Variables|UnitMovement|GetPrevious%20Transform)) (.location _transform)))) "1.000000,1.000000,1.000000"))
    (Components|Timeline|SetPlayRate _timeline_unitmovement (/ (Components|Timeline|GetTimelineLength _timeline_unitmovement) (Variables|UnitMovement|GetMoveDurationPerTile)))
    (bind (_direction _locationalpha _rotationalpha _jump) (Timeline|Timeline_UnitMovement PlayFromStart)
      (:Update
        (Transformation|SetActorLocationAndRotation (Math|Vector|MakeVector (.X (Math|Vector|BreakVector (Math|Vector|Lerp(Vector) (.location (Variables|UnitMovement|GetPrevious%20Transform)) (.location (Variables|UnitMovement|GetNext%20Transform)) _locationalpha))) (.Y (Math|Vector|BreakVector (Math|Vector|Lerp(Vector) (.location (Variables|UnitMovement|GetPrevious%20Transform)) (.location (Variables|UnitMovement|GetNext%20Transform)) _locationalpha))) (select (Math|Float|NearlyEqual(Float) (.z (.location (Variables|UnitMovement|GetPrevious%20Transform))) (.z (.location (Variables|UnitMovement|GetNext%20Transform))) 5.0) 0.0 _jump)) (Math|Rotator|Lerp(Rotator) (.rotation (Variables|UnitMovement|GetPrevious%20Transform)) (.rotation (Variables|UnitMovement|GetNext%20Transform)) _rotationalpha true)))
      (:Finished
        (Default|CallOnUnitReachedNewTile self (Utilities|Array|Get(acopy) (Variables|UnitMovement|GetCurrent%20Path%20To%20Follow)))
        (Utilities|Array|RemoveIndex (Variables|UnitMovement|GetCurrent%20Path%20To%20Follow))
        (CallFunction|ContinuetoFollowPath)))
    (else
      (Animation|SetAnimationState "NewEnumerator0")
      (Default|CallOnUnitFinishedWalking self))))

(event Custom|Debug_RespawnAferFewSeconds
  (Utilities|FlowControl|Delay 2.0)
  (Stats|SetCurrentHp (.HP_Max (Utilities|Struct|BreakS_UnitData_Stats (.Stats (Utilities|Struct|BreakS_UnitData (Variables|UnitData|GetUnit%20Data))))))
  (Animation|SetAnimationState "NewEnumerator5")
  (Default|EventUpdateHpBar (Variables|Default|GetHpBar)))

(event EventBeginPlay
  (Animation|SetAnimationState "NewEnumerator0")
  (bind _output_get (Variables|Default|SetHpBar (.AsWBP%20Hp%20Bar (Utilities|Casting|CastToWBP_HpBar (UserInterface|GetUserWidgetObject (Variables|Default|GetWidget_HpBar))))))
  (Default|EventSetUnit _output_get self))

(fn ConstructionScript
  (UnitData|SetUnitData (CallFunction|GetDefaultUnitDatafromUnitType (Variables|UnitData|GetUnitType))))

(fn UpdateVisualifHoveredorSelected
  (Rendering|Material|SetVectorParameterValueonMaterials (Variables|Default|GetSkeletalMesh) "ColorMultiply" (Math|Conversions|ToVector(LinearColor) (* (* (Math|Color|SelectColor "(R=0.400000,G=1.000000,B=0.700000,A=1.000000)" "(R=1.000000,G=1.000000,B=1.000000,A=1.000000)" (Variables|Hovered&Selected|GetIsSelected)) (Math|Float|SelectFloat 2.5 1.0 (Variables|Hovered&Selected|GetIsHovered))) (Math|Float|SelectFloat 2.5 1.0 (Variables|Hovered&Selected|GetIsSelected))))))

(fn SetIsHovered
  (params (Hovered :type Boolean))
  (Variables|Hovered&Selected|SetIsHovered Hovered)
  (Hovered&Selected|UpdateVisualifHoveredorSelected)
  (Default|CallOnUnitHoveredChanged self))

(fn SetIsSelected
  (params (Selected :type Boolean))
  (Variables|Hovered&Selected|SetIsSelected Selected)
  (Hovered&Selected|UpdateVisualifHoveredorSelected)
  (Default|CallOnUnitSelectedChanged self))

(fn SetUnitData
  (params (S_UnitData :type S%20Unit%20Data%20Structure%20%28by%20ref%29))
  (bind _skeletalmesh (Variables|Default|GetSkeletalMesh))
  (bind _output_get (Variables|UnitData|SetUnit%20Data S_UnitData))
  (Components|SkinnedMesh|SetSkinnedAssetandUpdate _skeletalmesh (.Mesh (Utilities|Struct|BreakS_UnitData_Assets (.Assets (Utilities|Struct|BreakS_UnitData _output_get)))) true)
  (Components|SkeletalMesh|SetAnimInstanceClass _skeletalmesh (.AnimBP (Utilities|Struct|BreakS_UnitData_Assets (.Assets (Utilities|Struct|BreakS_UnitData _output_get))))))

(fn SetAnimationState
  (params (State :type E_UnitAnimationState%20Enum :default "NewEnumerator0"))
  (Class|BPIUnitAnimation|SetUnitAnimationState(Message) (Components|SkeletalMesh|GetAnimInstance (Variables|Default|GetSkeletalMesh)) State))

(fn SetGrid
  (params (Grid :type BP%20Grid%20Object%20Reference))
  (bind _collision_lineofsight (Variables|Default|GetCollision_LineOfSight))
  (bind _mesh_teamindex (Variables|Default|GetMesh_TeamIndex))
  (Variables|Grid|SetGrid Grid)
  (Components|StaticMesh|SetStaticMesh _collision_lineofsight (.Mesh (Utilities|Struct|BreakS_GridShapeData (Default|GetCurrentShapeData Grid))))
  (Transformation|SetAbsolute _collision_lineofsight false true true)
  (Transformation|SetWorldScale3D _collision_lineofsight (Math|Vector|MakeVector (.X (Math|Vector|BreakVector (/ (Variables|/Game/AAA_Project/00_Core/Grid/BP_Grid.BP_Grid_C|GetGridTileSize Grid) (.MeshSize (Utilities|Struct|BreakS_GridShapeData (Default|GetCurrentShapeData Grid)))))) (.Y (Math|Vector|BreakVector (/ (Variables|/Game/AAA_Project/00_Core/Grid/BP_Grid.BP_Grid_C|GetGridTileSize Grid) (.MeshSize (Utilities|Struct|BreakS_GridShapeData (Default|GetCurrentShapeData Grid)))))) (.Z (Math|Vector|BreakVector (Transformation|GetWorldScale (Variables|Default|GetCollision_LineOfSight))))))
  (Transformation|SetWorldRotation _collision_lineofsight (Default|GetTileRotationfromGridIndex Grid (Variables|Grid|GetIndex)) false false)
  (Components|StaticMesh|SetStaticMesh _mesh_teamindex (.FlatMesh (Utilities|Struct|BreakS_GridShapeData (Default|GetCurrentShapeData Grid))))
  (Rendering|Material|SetMaterial _mesh_teamindex 0 (.FlatMaterial (Utilities|Struct|BreakS_GridShapeData (Default|GetCurrentShapeData Grid))))
  (Rendering|Material|SetScalarParameterValueonMaterials _mesh_teamindex "IsFilled" 1.0)
  (Transformation|SetAbsolute _mesh_teamindex false true true)
  (Transformation|SetWorldScale3D _mesh_teamindex (/ (Variables|/Game/AAA_Project/00_Core/Grid/BP_Grid.BP_Grid_C|GetGridTileSize (Variables|Grid|GetGrid)) (.MeshSize (Utilities|Struct|BreakS_GridShapeData (Default|GetCurrentShapeData Grid)))))
  (Transformation|SetWorldRotation _mesh_teamindex (Default|GetTileRotationfromGridIndex (Variables|Grid|GetGrid) (Variables|Grid|GetIndex)) false false)
  (Transformation|SetRelativeLocation _mesh_teamindex (Math|Vector|MakeVector 0.0 0.0 (+ (Variables|/Game/AAA_Project/00_Core/Grid/BP_GridVisual.BP_GridVisual_C|GetOffsetFromGround (Variables|/Game/AAA_Project/00_Core/Grid/BP_Grid.BP_Grid_C|GetGridVisual (Variables|Grid|GetGrid))) 5.0)) false false))

(fn SetGridIndex
  (params (Index :type Int%20Point%20Structure))
  (Variables|Grid|SetIndex Index)
  (Transformation|SetWorldRotation (Variables|Default|GetCollision_LineOfSight) (Default|GetTileRotationfromGridIndex (Variables|Grid|GetGrid) (Variables|Grid|GetIndex)) false false))

(fn UnitCastSpell
  (params (TargetIndex :type Int%20Point%20Structure) (SpellData :type S%20Spell%20Data%20Structure))
  (bind _returnvalue (Transformation|GetActorLocation))
  (bind _grid (Variables|Grid|GetGrid))
  (bind (_x _y) (Math|Vector|BreakVector _returnvalue))
  (bind _gridtiles (Variables|/Game/AAA_Project/00_Core/Grid/BP_Grid.BP_Grid_C|GetGridTiles _grid))
  (bind _value (Utilities|Map|Find _gridtiles TargetIndex))
  (bind _transform (Utilities|Struct|BreakS_TileData _value))
  (bind _location (Math|Transform|BreakTransform _transform))
  (bind (_x_2 _y_2) (Math|Vector|BreakVector _location))
  (Transformation|SetActorRotation (Math|Rotator|FindLookatRotation (Math|Vector|MakeVector _x _y 0.0) (Math|Vector|MakeVector _x_2 _y_2 0.0)))
  (Animation|SetAnimationState "NewEnumerator2")
  (Stats|ModifyCurrentAP (- 0 (Utilities|Struct|BreakS_SpellDate_Requirements (.Requirements (Utilities|Struct|BreakS_SpellData SpellData)))) true))

(fn ModifyCurrentHp
  (params (Modifier :type Integer))
  (Stats|SetCurrentHp (+ Modifier (.HP_Current (Utilities|Struct|BreakS_UnitData_Stats (.Stats (Utilities|Struct|BreakS_UnitData (Variables|UnitData|GetUnit%20Data))))))))

(fn SetCurrentHp
  (params (Hp :type Integer))
  (bind _structout (Utilities|Struct|SetmembersinS_UnitData_Stats (.Stats (Utilities|Struct|BreakS_UnitData (Variables|UnitData|GetUnit%20Data))) (Math|Integer|Clamp(Integer) Hp 0 (.HP_Max (Utilities|Struct|BreakS_UnitData_Stats (.Stats (Utilities|Struct|BreakS_UnitData (Variables|UnitData|GetUnit%20Data))))))))
  (Utilities|Struct|SetmembersinS_UnitData (Variables|UnitData|GetUnit%20Data) _structout)
  (Default|CallOnUnitsStatsChanged self))

(fn UnitHitbySpell
  (params (SpellImpactReal :type S%20Spell%20Data%20Impact%20Real%20Structure) (SpellAnimation :type BP%20Spell%20Animation%20Object%20Reference))
  (bind _modifier_hp (Utilities|Struct|BreakS_SpellData_Impact_Real SpellImpactReal))
  (Utilities|Map|Add (Variables|Default|GetIncomingSpellImpacts) SpellAnimation SpellImpactReal)
  (EventDispatchers|BindEventtoOnSpellAnimationHitTile SpellAnimation (EventDispatchers|CreateEvent :!event OnSpellAnimationHitTile))
  (if (!= _modifier_hp 0)
    (Stats|ModifyCurrentHp _modifier_hp)))

(fn OnSpellAnimationHitTile
  (params (SpellAnimation :type BP%20Spell%20Animation%20Object%20Reference) (TileIndex :type Int%20Point%20Structure))
  (bind _incomingspellimpacts (Variables|Default|GetIncomingSpellImpacts))
  (bind (_value _returnvalue) (Utilities|Map|Find _incomingspellimpacts SpellAnimation))
  (if (Class|KismetMathLibrary|EqualIntPointIntPoint (Variables|Grid|GetIndex) TileIndex)
    (if _returnvalue
      (LocalVariables|SetSpellImpactReal _value)
      (Utilities|Map|Remove (Variables|Default|GetIncomingSpellImpacts) SpellAnimation)
      (Default|EventUpdateHpBar (Variables|Default|GetHpBar))
      (if (!= (Utilities|Struct|BreakS_SpellData_Impact_Real (LocalVariables|GetSpellImpactReal)) 0)
        (Game|SpawnActorfromClass "/Game/AAA_Project/00_Core/Units/Widgets/BP_AnimatedNumber.BP_AnimatedNumber_C" (Math|Transform|MakeTransform (Transformation|GetActorLocation)) "Undefined" "MultiplyWithRoot" 0 (Utilities|Struct|BreakS_SpellData_Impact_Real (LocalVariables|GetSpellImpactReal)) "NewEnumerator0" 0)
        (if (< (Utilities|Struct|BreakS_SpellData_Impact_Real (LocalVariables|GetSpellImpactReal)) 0)
          (if (== (.HP_Current (Utilities|Struct|BreakS_UnitData_Stats (.Stats (Utilities|Struct|BreakS_UnitData (Variables|UnitData|GetUnit%20Data))))) 0)
            (if (Utilities|Enum|NotEqual(Enum) (Animation|GetAnimationState) "NewEnumerator4")
              (Animation|SetAnimationState "NewEnumerator4"))
            (else
              (Animation|SetAnimationState "NewEnumerator3"))))))))

(fn GetAnimationState
  (bind _state (Class|BPIUnitAnimation|GetUnitAnimationState(Message) (Components|SkeletalMesh|GetAnimInstance (Variables|Default|GetSkeletalMesh))))
  (return _state))

(fn SetTeamIndex
  (params (Index :type Integer))
  (Variables|Default|SetTeamIndex Index)
  (Class|ProgressBar|SetFillColorandOpacity (Variables|/Game/AAA_Project/00_Core/Units/Widgets/WBP_HpBar.WBP_HpBar_C|GetProgressBar_Hp (Variables|Default|GetHpBar)) (CallFunction|GetTeamColor (Variables|Default|GetTeamIndex)))
  (Rendering|Material|SetVectorParameterValueonMaterials (Variables|Default|GetMesh_TeamIndex) "Color" (Math|Conversions|ToVector(LinearColor) (CallFunction|GetTeamColor (Variables|Default|GetTeamIndex)))))

(fn CombatStarted
  (Development|PrintString "I'm in combat!")
  (Stats|ResetMp)
  (Stats|ResetAP))

(fn TurnStarted
  (Development|PrintString "It's my turn!"))

(fn TurnEnded
  (Development|PrintString "Sleep time!")
  (Stats|ResetMp)
  (Stats|ResetAP))

(fn CombatEnded
  (Development|PrintString "Vacation time!")
  (Stats|ResetMp)
  (Stats|ResetAP))

(fn SetCurrentMp
  (params (Mp :type Integer) (ShowNumber :type Boolean))
  (bind _unit_data (Variables|UnitData|GetUnit%20Data))
  (bind _stats (Utilities|Struct|BreakS_UnitData _unit_data))
  (bind (_validtiletypes _canmovediagonally _availablespells _hp_current _hp_max _mp_current _mp_max) (Utilities|Struct|BreakS_UnitData_Stats _stats))
  (LocalVariables|SetDifference (- Mp _mp_current))
  (bind _structout (Utilities|Struct|SetmembersinS_UnitData_Stats (.Stats (Utilities|Struct|BreakS_UnitData (Variables|UnitData|GetUnit%20Data))) (Math|Integer|Clamp(Integer) Mp 0 _mp_max)))
  (Utilities|Struct|SetmembersinS_UnitData (Variables|UnitData|GetUnit%20Data) _structout)
  (Default|CallOnUnitsStatsChanged self)
  (if (and ShowNumber (!= (LocalVariables|GetDifference) 0))
    (Game|SpawnActorfromClass "/Game/AAA_Project/00_Core/Units/Widgets/BP_AnimatedNumber.BP_AnimatedNumber_C" (Math|Transform|MakeTransform (Transformation|GetActorLocation)) "Undefined" "MultiplyWithRoot" 0 (LocalVariables|GetDifference) "NewEnumerator1" 0)))

(fn ModifyCurrentMp
  (params (Modifier :type Integer) (ShowNumber :type Boolean))
  (Stats|SetCurrentMp (+ Modifier (.MP_Current (Utilities|Struct|BreakS_UnitData_Stats (.Stats (Utilities|Struct|BreakS_UnitData (Variables|UnitData|GetUnit%20Data)))))) ShowNumber))

(fn ResetMp
  (Stats|SetCurrentMp (.MP_Max (Utilities|Struct|BreakS_UnitData_Stats (.Stats (Utilities|Struct|BreakS_UnitData (Variables|UnitData|GetUnit%20Data))))) true))

(fn SetCurrentAP
  (params (AP :type Integer) (ShowNumber :type Boolean))
  (bind _unit_data (Variables|UnitData|GetUnit%20Data))
  (bind _stats (Utilities|Struct|BreakS_UnitData _unit_data))
  (bind (_validtiletypes _canmovediagonally _availablespells _hp_current _hp_max _mp_current _mp_max _ap_current _ap_max) (Utilities|Struct|BreakS_UnitData_Stats _stats))
  (LocalVariables|SetDifference (- AP _ap_current))
  (bind _structout (Utilities|Struct|SetmembersinS_UnitData_Stats (.Stats (Utilities|Struct|BreakS_UnitData (Variables|UnitData|GetUnit%20Data))) (Math|Integer|Clamp(Integer) AP 0 _ap_max)))
  (Utilities|Struct|SetmembersinS_UnitData (Variables|UnitData|GetUnit%20Data) _structout)
  (Default|CallOnUnitsStatsChanged self)
  (if (and ShowNumber (!= (LocalVariables|GetDifference) 0))
    (Game|SpawnActorfromClass "/Game/AAA_Project/00_Core/Units/Widgets/BP_AnimatedNumber.BP_AnimatedNumber_C" (Math|Transform|MakeTransform (Transformation|GetActorLocation)) "Undefined" "MultiplyWithRoot" 0 (LocalVariables|GetDifference) "NewEnumerator2" 0)))

(fn ModifyCurrentAP
  (params (Modifier :type Integer) (ShowNumber :type Boolean))
  (Stats|SetCurrentAP (+ Modifier (.AP_Current (Utilities|Struct|BreakS_UnitData_Stats (.Stats (Utilities|Struct|BreakS_UnitData (Variables|UnitData|GetUnit%20Data)))))) ShowNumber))

(fn ResetAP
  (Stats|SetCurrentAP (.AP_Max (Utilities|Struct|BreakS_UnitData_Stats (.Stats (Utilities|Struct|BreakS_UnitData (Variables|UnitData|GetUnit%20Data))))) true))

(fn CanCastSpell
  (params (SpellData :type S%20Spell%20Data%20Structure))
  (if (Utilities|Array|ContainsItem (.AvailableSpells (Utilities|Struct|BreakS_UnitData_Stats (.Stats (Utilities|Struct|BreakS_UnitData (Variables|UnitData|GetUnit%20Data))))) (.Spell (Utilities|Struct|BreakS_SpellData SpellData)))
    (if (>= (.AP_Current (Utilities|Struct|BreakS_UnitData_Stats (.Stats (Utilities|Struct|BreakS_UnitData (Variables|UnitData|GetUnit%20Data))))) (Utilities|Struct|BreakS_SpellDate_Requirements (.Requirements (Utilities|Struct|BreakS_SpellData SpellData))))
      (return true)
      (else
        (return false)))
    (else
      (return false))))