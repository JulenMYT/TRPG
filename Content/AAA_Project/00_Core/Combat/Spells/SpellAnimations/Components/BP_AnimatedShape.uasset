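; BP_AnimatedShape is a short-lived spell animation actor that moves a colored mesh from an origin transform to a target transform.
; On BeginPlay it applies its mesh, material and color, then plays a timeline at a configurable rate.
; The timeline interpolates the transform and adds a curve-driven height offset above a fixed vertical lift.
; On finish it fires OnShapeAnimationCompleted, then destroys itself after a short delay.
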(event EventBeginPlay
  (bind _animatedshape (Variables|Default|GetAnimatedShape))
  (Components|StaticMesh|SetStaticMesh _animatedshape (Variables|Default|GetMesh))
  (Rendering|Material|SetMaterial _animatedshape 0 (Variables|Default|GetMaterial))
  (Rendering|Material|SetVectorParameterValueonMaterials _animatedshape "Color" (Math|Conversions|ToVector(LinearColor) (Variables|Default|GetColor)))
  (Components|Timeline|SetPlayRate (Variables|Default|GetTimeline_PlayAnimation) (Variables|Default|GetPlayRate))
  (bind (_direction _transformalhpa _heightoffset) (Timeline|Timeline_PlayAnimation PlayFromStart)
    (:Update
      (Transformation|SetActorTransform (Math|Transform|MakeTransform (+ (.location (Math|Transform|Lerp(Transform) (Variables|Default|GetOriginTransform) (Variables|Default|GetTargetTransform) _transformalhpa)) "0.000000,0.000000,100.000000" (Math|Vector|MakeVector 0.0 0.0 _heightoffset)) (.rotation (Math|Transform|Lerp(Transform) (Variables|Default|GetOriginTransform) (Variables|Default|GetTargetTransform) _transformalhpa)) (.scale (Math|Transform|Lerp(Transform) (Variables|Default|GetOriginTransform) (Variables|Default|GetTargetTransform) _transformalhpa)))))
    (:Finished
      (Default|CallOnShapeAnimationCompleted self)
      (Utilities|FlowControl|Delay 0.5)
      (Actor|DestroyActor))))

(fn ConstructionScript)