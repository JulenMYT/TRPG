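; Spell animation actor that shows a green, translucent wind gust moving from an origin transform to a target transform.
; Construction creates dynamic materials for two mesh slots, each a green tint with randomized brightness.
; On BeginPlay a timeline at a configurable play rate lerps the actor's transform, then signals shape animation completion and destroys the actor.
; The per-update scalar material write has no parameter name set.
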(event EventBeginPlay
  (Components|Timeline|SetPlayRate (Variables|Default|GetTimeline_PlayAnimation) (Variables|Default|GetPlayRate))
  (bind _transformalhpa (Timeline|Timeline_PlayAnimation PlayFromStart)
    (:Update
      (Transformation|SetActorTransform (Math|Transform|Lerp(Transform) (Variables|Default|GetOriginTransform) (Variables|Default|GetTargetTransform) _transformalhpa))
      (Rendering|Material|SetScalarParameterValueonMaterials (Variables|Default|GetAnimatedWindGust) "None" 0.0))
    (:Finished
      (Default|CallOnShapeAnimationCompleted self)
      (Actor|DestroyActor))))

(fn ConstructionScript
  (bind _returnvalue (Rendering|Material|CreateDynamicMaterialInstance (Variables|Default|GetAnimatedWindGust) 0 "/Game/AAA_Project/60_Environment/Materials/M_Translucent.M_Translucent" "None" :!class /Script/Engine.PrimitiveComponent))
  (Rendering|Material|SetVectorParameterValue _returnvalue "Color" (* "(R=0.098222,G=1.000000,B=0.072917,A=1.000000)" (Math|Random|RandomFloatinRange 0.8 1.5)) :!class /Script/Engine.MaterialInstanceDynamic)
  (bind _returnvalue_2 (Rendering|Material|CreateDynamicMaterialInstance (Variables|Default|GetAnimatedWindGust) 1 "/Game/AAA_Project/60_Environment/Materials/M_Translucent.M_Translucent" "None" :!class /Script/Engine.PrimitiveComponent))
  (Rendering|Material|SetVectorParameterValue _returnvalue_2 "Color" (* "(R=0.195244,G=0.791667,B=0.382867,A=1.000000)" (Math|Random|RandomFloatinRange 0.8 1.5)) :!class /Script/Engine.MaterialInstanceDynamic))