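; Spell animation actor for the Heal spell, showing a green effect on the target tile.
; The construction script tints six static meshes in three shades of green.
; When played, it moves to the target tile, then a timeline rotates and scales the AnimScale component while driving the meshes' material opacity.
; When the timeline finishes, it signals that the spell animation is complete.
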(event EventBeginPlay
  (|CallParentFunction) ; This node is disabled and will not be called.\nDrag off pins to build functionality.
)

(event Collision|EventActorBeginOverlap
  (params (OtherActor :type Actor%20Object%20Reference)))

(event EventTick
  (params (DeltaSeconds :type Float%20%28single-precision%29)))

(event EventEventPlaySpellAnimation
  (bind _anim_scale (Variables|Default|GetAnim_Scale))
  (Transformation|SetActorLocation (.Location (Math|Transform|BreakTransform (CallFunction|GetTileTransform (Variables|Default|GetTargetIndex)))) false false)
  (bind (_direction _opacity _rotation _scale) (Timeline|Timeline Play)
    (:Update
      (Transformation|SetRelativeRotation _anim_scale (Math|Rotator|MakeRotator 0.0 0.0 _rotation) false false)
      (Transformation|SetRelativeScale3D _anim_scale _scale)
      (Rendering|Material|SetScalarParameterValueonMaterials (Variables|Default|GetStaticMesh) "Opacity" _opacity))
    (:Finished
      (CallFunction|EventCompleteSpellAnimation))))

(fn ConstructionScript
  (|CallParentFunction)
  (Rendering|Material|SetVectorParameterValueonMaterials (Variables|Default|GetStaticMesh) "Color" (Math|Conversions|ToVector(LinearColor) "(R=0.200000,G=1.000000,B=0.200000,A=1.000000)"))
  (Rendering|Material|SetVectorParameterValueonMaterials (Variables|Default|GetStaticMesh1) "Color" (Math|Conversions|ToVector(LinearColor) "(R=0.100000,G=1.000000,B=0.100000,A=1.000000)"))
  (Rendering|Material|SetVectorParameterValueonMaterials (Variables|Default|GetStaticMesh2) "Color" (Math|Conversions|ToVector(LinearColor) "(R=0.000000,G=1.000000,B=0.000000,A=1.000000)")))