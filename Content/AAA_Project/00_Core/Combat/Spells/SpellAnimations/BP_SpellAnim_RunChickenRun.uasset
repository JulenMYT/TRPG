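; Spell animation Blueprint for Run Chicken Run, showing the spell's icon as an animated widget at the target tile.
; On play it moves to the target tile and sets the icon texture on its image widget, then a timeline drives the widget's height, draw size and opacity.
; It reports the tile hit once, early in the timeline, and completes the spell animation when the timeline finishes.
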(event EventBeginPlay
  (|CallParentFunction) ; This node is disabled and will not be called.\nDrag off pins to build functionality.
)

(event EventEventPlaySpellAnimation
  (bind _widget (Variables|Default|GetWidget))
  (Transformation|SetActorLocation (.Location (Math|Transform|BreakTransform (CallFunction|GetTileTransform (Variables|Default|GetTargetIndex)))) false false)
  (bind _output_get (Variables|Default|SetW_Image (.AsW%20Image (Utilities|Casting|CastToW_Image (UserInterface|GetUserWidgetObject (Variables|Default|GetWidget))))))
  (Appearance|SetBrushfromTexture (Variables|/Game/AAA_Project/00_Core/Combat/Spells/SpellAnimations/Components/W_Image.W_Image_C|GetImage_Component _output_get) "/Game/AAA_Project/00_Core/Combat/Spells/SpellAnimations/Assets/Icon_RunChickenRun_NoBackground.Icon_RunChickenRun_NoBackground" false)
  (bind (_direction _locationz _drawsize _opacity) (Timeline|Timeline_RunChickenRun PlayFromStart)
    (:Update
      (Transformation|SetRelativeLocation _widget (Math|Vector|MakeVector 0.0 0.0 _locationz) false false)
      (Class|WidgetComponent|SetDrawSize _widget (Math|Vector2D|MakeVector2D _drawsize _drawsize))
      (Widget|SetRenderOpacity (Variables|Default|GetW_Image) _opacity)
      (if (>= (Components|Timeline|GetPlaybackPosition (Variables|Default|GetTimeline_RunChickenRun)) 0.2)
        (Utilities|FlowControl|DoOnce false
          (:Completed
            (Default|CallOnSpellAnimationHitTile self (Variables|Default|GetTargetIndex))))))
    (:Finished
      (CallFunction|EventCompleteSpellAnimation))))

(fn ConstructionScript
  (|CallParentFunction))