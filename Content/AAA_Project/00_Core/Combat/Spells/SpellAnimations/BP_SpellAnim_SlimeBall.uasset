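; Spell animation actor for the Slime Ball spell, showing a green projectile flying from an origin tile to a target tile.
; A timeline drives position along an arc, plus the scale and opacity of three meshes tinted in different greens at construction.
; Partway through playback it notifies a hit on every attacked tile once, then completes the spell animation when the timeline finishes.
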(event EventBeginPlay
  (|CallParentFunction) ; This node is disabled and will not be called.\nDrag off pins to build functionality.
)

(event EventEventPlaySpellAnimation
  (Transformation|SetActorLocation (.Location (Math|Transform|BreakTransform (CallFunction|GetTileTransform (Variables|Default|GetTargetIndex)))) false false)
  (bind (_direction _opacity _scale _locationalpha _locationz) (Timeline|Timeline_SlimeBall Play)
    (:Update
      (Transformation|SetActorLocation (+ (Math|Vector|Lerp(Vector) (.Location (Math|Transform|BreakTransform (CallFunction|GetTileTransform (Variables|Default|GetOrigin%20Index)))) (.Location (Math|Transform|BreakTransform (CallFunction|GetTileTransform (Variables|Default|GetTargetIndex)))) _locationalpha) (Math|Vector|MakeVector 0.0 0.0 _locationz)) false false)
      (Rendering|Material|SetScalarParameterValueonMaterials (Variables|Default|GetStaticMesh) "Opacity" _opacity)
      (Transformation|SetRelativeScale3D (Variables|Default|GetAnim_Scale) _scale)
      (if (>= (Components|Timeline|GetPlaybackPosition (Variables|Default|GetTimeline_SlimeBall)) 0.55)
        (Utilities|FlowControl|DoOnce false
          (:Completed
            (for _array_element (Variables|Default|GetAttackedIndexes)
              (Default|CallOnSpellAnimationHitTile self _array_element))))))
    (:Finished
      (CallFunction|EventCompleteSpellAnimation))))

(fn ConstructionScript
  (|CallParentFunction)
  (Rendering|Material|SetVectorParameterValueonMaterials (Variables|Default|GetStaticMesh) "Color" (Math|Conversions|ToVector(LinearColor) "(R=0.051042,G=0.255208,B=0.051042,A=1.000000)"))
  (Rendering|Material|SetVectorParameterValueonMaterials (Variables|Default|GetStaticMesh1) "Color" (Math|Conversions|ToVector(LinearColor) "(R=0.052604,G=0.526042,B=0.052604,A=1.000000)"))
  (Rendering|Material|SetVectorParameterValueonMaterials (Variables|Default|GetStaticMesh2) "Color" (Math|Conversions|ToVector(LinearColor) "(R=0.000000,G=0.859375,B=0.000000,A=1.000000)")))