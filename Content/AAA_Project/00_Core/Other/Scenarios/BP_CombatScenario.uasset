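; BP_CombatScenario is a placeable combat scenario that starts a grid battle on play and restarts it with reset unit HP whenever it ends.
; In the editor, its construction script centers and spawns the grid on the actor and records each unit's tile from its placement.
; Helper functions, not called here, derive teams from "Team<N>_" unit names and assign teams other than index 0 to AI.
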(event Custom|OnCombatEnded
  (if (== (Variables|/Game/AAA_Project/00_Core/Combat/BP_CombatSytem.BP_CombatSytem_C|GetObjectThatStartedCombat (Variables|Default|GetCombatSystem)) self)
    (for _array_element (.UnitTeams (Utilities|Struct|BreakS_QuickCombat_UnitTeams (Variables|Default|GetUnitsData)))
      (for _array_element_2 (Utilities|Struct|BreakS_UnitArray _array_element)
        (Default|ResetHp _array_element_2)))
    (Default|QuickStartCombat (Variables|Default|GetCombatSystem) (Variables|Default|GetGridData) (Variables|Default|GetUnitsData) self)))

(event EventBeginPlay
  (Utilities|FlowControl|Delay 0.4)
  (EventDispatchers|BindEventtoOnCombatEnded (Variables|Default|GetCombatSystem) (delegate Custom|OnCombatEnded))
  (Default|QuickStartCombat (Variables|Default|GetCombatSystem) (Variables|Default|GetGridData) (Variables|Default|GetUnitsData) self))

(fn ConstructionScript
  (if (not (CallFunction|IsinGame))
    (Utilities|Struct|SetmembersinS_QuickCombat_Grid (Variables|Default|GetGridData) (Transformation|GetActorLocation))
    (CallFunction|SpawnGrid)
    (CallFunction|BuildDesiredGridIndexesBasedonUnitLocations)))

(fn BuildTeamsBasedonUnitNames
  (bind _outactors (Actor|GetAllActorsOfClass "/Game/AAA_Project/00_Core/Units/BP_Unit.BP_Unit_C"))
  (for _array_element _outactors
    (LocalVariables|SetUnit _array_element)
    (LocalVariables|SetTeamIndex (Math|Conversions|ToInteger(Byte) (.LeftS (Utilities|String|Split (.RightS (Utilities|String|Split (Utilities|GetDisplayName (LocalVariables|GetUnit)) "Team")) "_"))))
    (if (< (Utilities|Array|Length (LocalVariables|GetUnitTeams)) (+ (LocalVariables|GetTeamIndex) 1))
      (Utilities|Array|Resize (LocalVariables|GetUnitTeams) (+ (LocalVariables|GetTeamIndex) 1)))
    (Utilities|Array|Add (Utilities|Struct|BreakS_UnitArray (Utilities|Array|Get(acopy) (LocalVariables|GetUnitTeams) (LocalVariables|GetTeamIndex))) (LocalVariables|GetUnit)))
  (Utilities|Array|RemoveItem :TargetArray (LocalVariables|GetUnitTeams))
  (Utilities|Struct|SetmembersinS_QuickCombat_UnitTeams (Variables|Default|GetUnitsData) (LocalVariables|GetUnitTeams)))

(fn BuildAiListBasedonTeamIndexes
  (for (_array_element _array_index) (.UnitTeams (Utilities|Struct|BreakS_QuickCombat_UnitTeams (Variables|Default|GetUnitsData)))
    (if (!= _array_index 0)
      (Utilities|Array|AppendArray (LocalVariables|GetAis) (Utilities|Struct|BreakS_UnitArray _array_element))))
  (Utilities|Struct|SetmembersinS_QuickCombat_UnitTeams (Variables|Default|GetUnitsData) (LocalVariables|GetAis)))

(fn BuildDesiredGridIndexesBasedonUnitLocations
  (for _array_element (.UnitTeams (Utilities|Struct|BreakS_QuickCombat_UnitTeams (Variables|Default|GetUnitsData)))
    (for _array_element_2 (Utilities|Struct|BreakS_UnitArray _array_element)
      (bind _index (Default|GetTileIndexfromWorldLocation (Variables|/Game/AAA_Project/00_Core/Combat/BP_CombatSytem.BP_CombatSytem_C|GetGrid (Variables|Default|GetCombatSystem)) (Transformation|GetActorLocation _array_element_2)))
      (Utilities|Map|Add (LocalVariables|GetDesiredIndexes) _array_element_2 _index)))
  (Utilities|Struct|SetmembersinS_QuickCombat_UnitTeams (Variables|Default|GetUnitsData) (LocalVariables|GetDesiredIndexes)))

(fn SpawnGrid
  (bind _combatsystem (Variables|Default|GetCombatSystem))
  (bind _griddata (Variables|Default|GetGridData))
  (bind (_generategridbeforestartingcombat _centerlocation _tilesize _tilecount _shape _useenvironment) (Utilities|Struct|BreakS_QuickCombat_Grid _griddata))
  (bind _grid (Variables|/Game/AAA_Project/00_Core/Combat/BP_CombatSytem.BP_CombatSytem_C|GetGrid _combatsystem))
  (Utilities|IsValid _combatsystem
    (:Is%20Valid
      (Utilities|IsValid _grid
        (:Is%20Valid
          (Default|SpawnGrid _grid _centerlocation _tilesize _tilecount _shape _useenvironment))))))