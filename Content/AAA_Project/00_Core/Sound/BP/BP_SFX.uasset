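; BP_SFX is a sound-effect actor that plays a random clip from an array of sound waves through its audio component.
; The construction script applies the base volume and toggles spatialization for 2D or 3D playback.
; It can play on BeginPlay and, when looping, waits a random delay after each clip finishes before playing another random pick.
; Functions also expose stop, volume and spatialization control.
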(event OnAudioFinished(Audio)
  (if (Variables|Loop|GetIsLooping)
    (Utilities|FlowControl|Delay (Math|Random|RandomFloatinRange (Variables|Loop|GetMinLoopTime) (Variables|Loop|GetMaxLoopTime)))
    (CallFunction|PlayRandomSFX)))

(event EventBeginPlay
  (if (Variables|Default|GetPlayOnAwake)
    (CallFunction|PlayRandomSFX)))

(fn ConstructionScript
  (CallFunction|SetVolume (Variables|Default|GetBase%20Volume%20Multiplier))
  (if (Variables|Default|GetIs3D)
    (CallFunction|Set3DSound)
    (else
      (CallFunction|Set2DSound))))

(fn PlayRandomSFX
  (bind _audio (Variables|Default|GetAudio))
  (Audio|Components|Audio|SetSound _audio (.OutItem (Utilities|Array|Random (Variables|Default|GetSound%20Wave%20Array))))
  (Audio|Components|Audio|Play _audio 0.0))

(fn StopSFX
  (Audio|Components|Audio|Stop (Variables|Default|GetAudio)))

(fn SetVolume
  (params (VolumeMultiplier :type Float%20%28single-precision%29))
  (Audio|Components|Audio|SetVolumeMultiplier (Variables|Default|GetAudio) VolumeMultiplier :!class /Script/Engine.AudioComponent))

(fn Set2DSound
  (Variables|/Script/Engine.AudioComponent|SetbAllowSpatialization (Variables|Default|GetAudio) false))

(fn Set3DSound
  (Variables|/Script/Engine.AudioComponent|SetbAllowSpatialization (Variables|Default|GetAudio) true))