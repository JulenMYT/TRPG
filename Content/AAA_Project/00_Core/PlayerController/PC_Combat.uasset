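; Player controller for combat that handles movement input and ends the battle from hardcoded numpad keys.
; BeginPlay adds the combat Enhanced Input mapping context, and IA_Move moves the controlled pawn along world X/Y, independent of camera rotation.
; NumPad 0 and 1 show the lose or win widget, then after a short delay load the main menu or Level01 respectively.
; A BattleEnded flag ensures only one outcome fires.
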(event Input|EnhancedActionEvents|EnhancedInputActionIA_Move
  (params (ActionValue :type Vector%202D%20Structure) (ElapsedSeconds :type Float%20%28double-precision%29) (TriggeredSeconds :type Float%20%28double-precision%29) (InputAction :type Input%20Action%20Object%20Reference :default "/Game/AAA_Project/00_Core/Inputs/IA_Move.IA_Move"))
  (bind (_x _y) (Math|Vector2D|BreakVector2D ActionValue))
  (Pawn|Input|AddMovementInput (Pawn|GetControlledPawn) (Math|Vector|MakeVector _x _y 0.0) 1.0 false))

(event EventBeginPlay
  (Input|AddMappingContext (PlayerController|LocalPlayerSubsystems|GetEnhancedInputLocalPlayerSubsystem) "/Game/AAA_Project/00_Core/Inputs/IMC_Combat.IMC_Combat" 0 "(bIgnoreAllPressedKeysUntilRelease=True,bForceImmediately=False,bNotifyUserSettings=False)"))

(event Input|KeyboardEvents|NumPadZero
  (params (Key :type Key%20Structure :default "None"))
  (:Pressed
    (if (not (Variables|Default|GetBattleEnded))
      (Variables|Default|SetBattleEnded true)
      (bind _returnvalue (UserInterface|CreateWidget "/Game/AAA_Project/40_UI/EndBattleScreen/WBP_Lose.WBP_Lose_C" self))
      (UserInterface|Viewport|AddtoViewport _returnvalue 0)
      (Utilities|FlowControl|Delay 2.0)
      (Game|OpenLevel(byObjectReference) "/Game/AAA_Project/60_Environment/Levels/L_MainMenu.L_MainMenu"))))

(event Input|KeyboardEvents|NumPadOne
  (params (Key :type Key%20Structure :default "None"))
  (:Pressed
    (if (not (Variables|Default|GetBattleEnded))
      (Variables|Default|SetBattleEnded true)
      (bind _returnvalue (UserInterface|CreateWidget "/Game/AAA_Project/40_UI/EndBattleScreen/WBP_Win.WBP_Win_C" self))
      (UserInterface|Viewport|AddtoViewport _returnvalue 0)
      (Utilities|FlowControl|Delay 2.0)
      (Game|OpenLevel(byObjectReference) "/Game/AAA_Project/60_Environment/Levels/L_Level01.L_Level01"))))

(fn ConstructionScript)