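; PC_Exploration is the player controller for exploration, handling movement and interaction input and the interaction popup.
; On BeginPlay it adds the IMC_Exploration mapping context and creates a hidden WBP_Popup, toggled through ShowInteractionWidget and HideInteractionWidget.
; IA_Move feeds world-axis movement, not camera-relative, to the controlled pawn.
; IA_Interaction casts that pawn to BP_PlayerExploration and calls its Interact function.
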(event Input|EnhancedActionEvents|EnhancedInputActionIA_Move
  (params (ActionValue :type Vector%202D%20Structure) (ElapsedSeconds :type Float%20%28double-precision%29) (TriggeredSeconds :type Float%20%28double-precision%29) (InputAction :type Input%20Action%20Object%20Reference :default "/Game/AAA_Project/00_Core/Inputs/IA_Move.IA_Move"))
  (bind (_x _y) (Math|Vector2D|BreakVector2D ActionValue))
  (Pawn|Input|AddMovementInput (Pawn|GetControlledPawn) (Math|Vector|MakeVector _x _y 0.0) 1.0 false))

(event Input|EnhancedActionEvents|EnhancedInputActionIA_Interaction
  (params (ActionValue :type Boolean) (ElapsedSeconds :type Float%20%28double-precision%29) (TriggeredSeconds :type Float%20%28double-precision%29) (InputAction :type Input%20Action%20Object%20Reference :default "/Game/AAA_Project/00_Core/Inputs/IA_Interaction.IA_Interaction"))
  (bind _asbp_player_exploration (Utilities|Casting|CastToBP_PlayerExploration (Pawn|GetControlledPawn)))
  (Default|Interact _asbp_player_exploration))

(event EventBeginPlay
  (Input|AddMappingContext (PlayerController|LocalPlayerSubsystems|GetEnhancedInputLocalPlayerSubsystem) "/Game/AAA_Project/00_Core/Inputs/IMC_Exploration.IMC_Exploration" 0 "(bIgnoreAllPressedKeysUntilRelease=True,bForceImmediately=False,bNotifyUserSettings=False)")
  (bind _returnvalue (UserInterface|CreateWidget "/Game/AAA_Project/40_UI/HUD/WBP_Popup.WBP_Popup_C" (Game|GetPlayerController 0)))
  (Variables|Default|SetInteractionWidget _returnvalue)
  (UserInterface|Viewport|AddtoViewport _returnvalue 0)
  (Widget|SetVisibility _returnvalue "Hidden"))

(fn ConstructionScript)

(fn ShowInteractionWidget
  (Widget|SetVisibility (Variables|Default|GetInteractionWidget) "Visible"))

(fn HideInteractionWidget
  (Widget|SetVisibility (Variables|Default|GetInteractionWidget) "Hidden"))