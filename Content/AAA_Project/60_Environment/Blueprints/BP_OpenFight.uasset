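; BP_OpenFight is an interactable environment Blueprint that sends the player from exploration into a fight level.
; Entering and exiting its trigger shows or hides the interaction widget through the PC_Exploration player controller.
; Interacting adds a WBP_Dialogue widget to the viewport, waits on a fixed delay, then calls LoadFight, which opens the level referenced by LevelToLoad.
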(event EventEnterTrigger
  (bind _aspc_exploration (Utilities|Casting|CastToPC_Exploration (Game|GetPlayerController 0)))
  (Default|ShowInteractionWidget _aspc_exploration))

(event EventExitTrigger
  (bind _aspc_exploration (Utilities|Casting|CastToPC_Exploration (Game|GetPlayerController 0)))
  (Default|HideInteractionWidget _aspc_exploration))

(event EventInteract
  (bind _returnvalue (UserInterface|CreateWidget "/Game/AAA_Project/40_UI/Dialogue/WBP_Dialogue.WBP_Dialogue_C"))
  (UserInterface|Viewport|AddtoViewport _returnvalue 0)
  (Utilities|FlowControl|Delay 3.0)
  (CallFunction|LoadFight))

(fn ConstructionScript)

(fn LoadFight
  (Game|OpenLevel(byObjectReference) (Variables|Default|GetLevelToLoad)))